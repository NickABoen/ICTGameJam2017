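; EnemyPixel is an enemy actor that chases the player and respawns characters it touches.
; Each Tick it moves straight toward its Player reference by Speed units, with no sweep and no delta-time scaling, so its pace depends on frame rate.
; On overlap, it looks up a RespawnComponent on the other actor and, if one exists, calls RespawnCharacter on it.
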(event `self.ReceiveActorBeginOverlap`
  (params (OtherActor :type "Actor Object Reference"))
  (bind _asrespawn_component (cast `RespawnComponent` (`self.GetComponentByClass` OtherActor "/Script/ICTGameJam2017.RespawnComponent")))
  (`RespawnComponent.RespawnCharacter` _asrespawn_component))

(event `self.ReceiveTick`
  (params (DeltaSeconds :type "Float (single-precision)"))
  (`self.K2_SetActorLocation` (+ (`self.K2_GetActorLocation`) (* (`KismetMathLibrary.Normal` (- (`self.K2_GetActorLocation` (`self.Player`)) (`self.K2_GetActorLocation`))) (`self.Speed`)))))

(fn `UserConstructionScript`)